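; BPGA_Teleport is a Gameplay Ability that, despite its name, spawns a testing dummy at a targeted point rather than moving the player.
; On activation, WaitTargetData runs a user-confirmed TestTrace targeting actor from the owning character, with debug enabled.
; Valid data commits the ability; only authority spawns BP_TestingDummy slightly above the hit, then both sides end the ability.
; Cancelled targeting or failed commit cancels it.
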(event `self.K2_ActivateAbility`
  (bind _owning (`self.Owning`))
  (bind (_locationtype _literaltransform _sourceactor _sourcecomponent _sourceability _sourcesocketname) (break `GameplayAbilityTargetingLocationInfo` (`self.MakeTargetLocationInfoFromOwnerActor`)))
  (`KismetSystemLibrary.PrintString` "Hello")
  (bind _asunplayer_character (cast `UNPlayerCharacter` (`self.GetAvatarActorFromActorInfo`)))
  (set `self.Owning` _asunplayer_character)
  (`KismetSystemLibrary.PrintString` "Start AT")
  (bind (_asynctaskproxy _data) (`AbilityTask_WaitTargetData.WaitTargetData` "None" "UserConfirmed" "/Game/Blueprint/GA/TestTrace.TestTrace_C" 2000.0 0.0 2000.0 (struct :`Name` "BlockAllDynamic") true (make `GameplayAbilityTargetingLocationInfo` _locationtype (`KismetMathLibrary.MakeTransform` (+ (`Actor.GetActorForwardVector` (`self.Owning`)) (.location _literaltransform)) (.rotation _literaltransform) (.scale _literaltransform)) _sourceactor _sourcecomponent _sourceability _sourcesocketname) (struct) null (struct) true)
    (:`ValidData`
      (`KismetSystemLibrary.PrintString` "end AT")
      (bind _returnvalue (`self.K2_CommitAbility`))
      (if _returnvalue
        (if (`Actor.HasAuthority` (`self.Owning`))
          (bind (_returnvalue_bblockinghit _returnvalue_binitialoverlap _returnvalue_time _returnvalue_distance _returnvalue_location) (`GameplayStatics.BreakHitResult` (`AbilitySystemBlueprintLibrary.GetHitResultFromTargetData` _data)))
          (`|SpawnActorFromClass` "/Game/Blueprint/BP_TestingDummy.BP_TestingDummy_C" (`KismetMathLibrary.MakeTransform` (+ _returnvalue_location (0.0 0.0 10.0))) "Undefined" "MultiplyWithRoot" _owning _owning)
          (`KismetSystemLibrary.PrintString` "Final")
          (`self.K2_EndAbility`)
          (else
            (`KismetSystemLibrary.PrintString` "End")
            (`self.K2_EndAbility`)))
        (else
          (`KismetSystemLibrary.PrintString` "cancel" :!label _label)
          (`self.K2_CancelAbility`))))
    (:`Cancelled`
      (goto _label))))